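; BP_GridAnchor is a scene component that aligns its owning actor to the tile grid of BP_GridManager_Custom.
; An external construction event conditionally snaps the component to the tile traced from the owner's location and stores that tile's GridIndex.
; PlaceActorAtAnchor traces from the component's own position, adds AnchorOffset, moves the owner there and zeroes the component's relative location.
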(event Custom|ExternalConstuctionScript
  (bind _returnvalue (Components|GetOwner))
  (bind _returnvalue_2 (Actor|GetActorOfClass "/Game/AdvancedTurnBasedTileToolkit/Core/Grid/BP_GridManager_Custom.BP_GridManager_Custom_C"))
  (Utilities|IsValid _returnvalue_2
    (:Is%20Valid
      (if (or (Variables|Default|GetbIgnoreSnapToCustomGrid) (not (Default|CheckforCompileError _returnvalue_2)))
        _
        (else
          (bind _snaplocation (Default|FindClosestTiletoSnaptoTrace _returnvalue_2 (Transformation|GetActorLocation _returnvalue) (Utilities|Array|MakeArray _returnvalue)))
          (Transformation|SetWorldLocation self _snaplocation false false)))
      (Variables|Default|SetGridIndex (.Index (Default|ConvertLocationtoIndex3D _returnvalue_2 _snaplocation))))))

(fn PlaceActoratAnchor
  (bind _returnvalue (Actor|GetActorOfClass "/Game/AdvancedTurnBasedTileToolkit/Core/Grid/BP_GridManager_Custom.BP_GridManager_Custom_C"))
  (bind _snaplocation (Default|FindClosestTiletoSnaptoTrace _returnvalue (Transformation|GetWorldLocation) (Utilities|Array|MakeArray (Components|GetOwner))))
  (Transformation|SetWorldLocation (+ _snaplocation (Variables|Default|GetAnchorOffset)) false false)
  (Transformation|SetActorLocation (Components|GetOwner) (Transformation|GetWorldLocation) false false)
  (Transformation|SetRelativeLocation "0, 0, 0" false false)
  (return))