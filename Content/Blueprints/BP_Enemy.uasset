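; BP_Enemy is an enemy character that faces the player on BeginPlay and reports its death to BP_GameMode's NPC kill count.
; Its StatBar widget gets a red health fill and is made visible when the parent's damage event fires.
; EquipWeapon resolves a skeletal mesh from an asset path through the Asset Registry and attaches it to the right-hand weapon socket as a spawned actor, destroyed on replacement or EndPlay.
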(event EventBeginPlay
  (|CallParentFunction)
  (CallFunction|LookatPlayerCharacter)
  (Class|ProgressBar|SetFillColorandOpacity (Variables|/Game/UI/StatBar.StatBar_C|GetHealthGauge (.AsStat%20Bar (Utilities|Casting|CastToStatBar (UserInterface|GetUserWidgetObject (Variables|Default|GetStatBar))))) "(R=0.627604,G=0.003269,B=0.003269,A=1.000000)"))

(event EventEndPlay
  (params (EndPlayReason :type EEndPlayReason%20Enum :default "Destroyed"))
  (bind _weaponactor (Variables|Default|GetWeaponActor))
  (if (Utilities|IsValid _weaponactor)
    (Actor|DestroyActor _weaponactor)))

(event EventOnDamaged
  (params (DamageAmount :type Float%20%28single-precision%29) (HitInfo :type Hit%20Result%20Structure%20%28by%20ref%29) (DamageTags :type Gameplay%20Tag%20Container%20Structure%20%28by%20ref%29) (InstigatorCharacter :type Character%20Base%20Object%20Reference) (DamageCauser :type Actor%20Object%20Reference))
  (|CallParentFunction DamageAmount HitInfo DamageTags InstigatorCharacter DamageCauser)
  (Rendering|SetVisibility (Variables|Default|GetStatBar) true false))

(fn ConstructionScript)

(fn EquipWeapon
  (params (AssetPath :type String))
  (Utilities|IsValid (Variables|Default|GetWeaponActor)
    (:Is%20Valid
      (Actor|DestroyActor (Variables|Default|GetWeaponActor)))
    (:Is%20Not%20Valid
      _))
  (bind _returnvalue (Class|AssetRegistry|GetAssetbyObjectPath (Class|AssetRegistryHelpers|GetAssetRegistry) (Utilities|String|StringToName AssetPath) false))
  (bind _asskeletal_mesh (Utilities|Casting|CastToSkeletalMesh (Class|AssetRegistryHelpers|GetAsset _returnvalue)))
  (if (Utilities|IsValid _asskeletal_mesh)
    (bind _returnvalue_2 (Class|MovieSceneTransformOrigin|GetTransformOrigin(Message) (Variables|Character|GetCharacterMovement)))
    (bind _returnvalue_3 (Game|SpawnActorfromClass "/Script/Engine.SkeletalMeshActor" _returnvalue_2 "Undefined" 0 0))
    (Variables|Default|SetWeaponActor _returnvalue_3)
    (Class|SkinnedMeshComponent|SetSkeletalMesh (Variables|/Script/Engine.SkeletalMeshActor|GetSkeletalMeshComponent _returnvalue_3) _asskeletal_mesh true)
    (Transformation|AttachComponentToComponent _returnvalue_3 (Variables|Character|GetMesh) "b_MF_Weapon_R" "SnapToTarget" "SnapToTarget" "KeepWorld" true)))

(fn OnDie
  (bind _asbp_game_mode (Utilities|Casting|CastToBP_GameMode (Game|GetGameMode)))
  (Default|IncreaseNPCKillCount _asbp_game_mode 0.0))

(fn LookatPlayerCharacter
  (Transformation|SetActorRotation (Math|Rotator|MakeRotator 0.0 0.0 (.Yaw (Math|Rotator|BreakRotator (Math|Rotator|FindLookatRotation (Transformation|GetActorLocation) (Transformation|GetActorLocation (CallFunction|GetPlayerCharacterBP))))))))