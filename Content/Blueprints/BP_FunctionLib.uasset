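; Blueprint function library of shortcuts to the game's core Blueprint classes and a cursor picking helper.
; Getters cast the game mode, player 0's controller as either the standard or card variant, and that player's controlled character.
; GetPickingPoint traces visibility under the cursor, picks a random navigable location within a small radius of the hit, and returns it raised along Z.
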(fn GetGameModeBP
  (bind _asbp_gamemode (Utilities|Casting|CastToBP_GameMode (Game|GetGameMode))
    (:then
      _)
    (:CastFailed
      _))
  (return _asbp_gamemode))

(fn GetPlayerContollerBP
  (bind _asbp_player_controller (Utilities|Casting|CastToBP_PlayerController (Game|GetPlayerController 0)))
  (return _asbp_player_controller))

(fn GetPlayerCharacterBP
  (return (.AsBP%20Player%20Character (Utilities|Casting|CastToBP_PlayerCharacter (Pawn|GetControlledPawn (.AsBP%20Player%20Controller (Utilities|Casting|CastToBP_PlayerController (Game|GetPlayerController 0))))))))

(fn GetPlayerControllerCardBP
  (bind _asbp_player_controller_card (Utilities|Casting|CastToBP_PlayerControllerCard (Game|GetPlayerController 0)))
  (return _asbp_player_controller_card))

(fn GetPickingPoint
  (bind _randomlocation (Class|NavigationSystemV1|GetRandomLocationinNavigableRadius 0 (.ImpactPoint (Collision|BreakHitResult (.HitResult (Game|Player|GetHitResultUnderCursorbyChannel (CallFunction|GetPlayerContollerBP) "TraceTypeQuery1" true)))) 5e+01 0 0))
  (return (Math|Vector|MakeVector (.X (Math|Vector|BreakVector (.Location (Math|Transform|BreakTransform (Math|Conversions|ToTransform(Vector) _randomlocation))))) (.Y (Math|Vector|BreakVector (.Location (Math|Transform|BreakTransform (Math|Conversions|ToTransform(Vector) _randomlocation))))) (+ (.Z (Math|Vector|BreakVector (.Location (Math|Transform|BreakTransform (Math|Conversions|ToTransform(Vector) _randomlocation))))) 1e+02))))