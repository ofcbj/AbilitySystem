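; CardDrag is the drag-and-drop operation for dragging a card out of the player's hand.
; On drag cancel, a card over the use area is used and removed from the hand through its card manager.
; Otherwise, the card jumps to the pointer position via render translation, becomes visible and interpolates back to its home transform.
; A successful drop only prints a debug string, so card play happens in the cancel path.
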(event EventDrop
  (params (PointerEvent :type Pointer%20Event%20Structure%20%28by%20ref%29))
  (Development|PrintString 0 "drop"))

(event EventDragCancelled
  (params (PointerEvent :type Pointer%20Event%20Structure%20%28by%20ref%29))
  (bind _returnvalue (Class|KismetInputLibrary|PointerEventGetScreenSpacePosition PointerEvent))
  (bind _cardinhand (Variables|Default|GetCardInHand))
  (bind _cardinhand_2 (Variables|Default|GetCardInHand))
  (bind _cardinhand_3 (Variables|Default|GetCardInHand))
  (bind _uiparent (Variables|/Game/CCGToolkit/Blueprints/Widgets/Gameplay/CardWidget.CardWidget_C|GetUIParent _cardinhand))
  (bind _returnvalue_2 (Class|Widget|GetCachedGeometry _uiparent))
  (bind _returnvalue_3 (Class|SlateBlueprintLibrary|GetLocalSize _returnvalue_2))
  (bind _returnvalue_4 (Class|SlateBlueprintLibrary|AbsolutetoLocal _returnvalue_2 _returnvalue))
  (bind (_x _y) (Math|Vector2D|BreakVector2D _returnvalue_3))
  (bind (_x_2 _y_2) (Math|Vector2D|BreakVector2D _returnvalue_4))
  (bind _inusearea (Default|IsUseArea (Variables|/Game/CCGToolkit/Blueprints/Widgets/Gameplay/CardWidget.CardWidget_C|GetDragCard _cardinhand)))
  (if _inusearea
    (Default|Use _cardinhand_3)
    (Default|RemoveCardWidgetfromHand (Variables|/Game/CCGToolkit/Blueprints/Widgets/Gameplay/CardWidget.CardWidget_C|GetCardManager_Ref _cardinhand_3) _cardinhand_3 0 false)
    (else
      (Variables|/Game/CCGToolkit/Blueprints/Widgets/Gameplay/CardWidget.CardWidget_C|SetMoveComponent _cardinhand_3 _cardinhand_3)
      (Class|Widget|SetRenderTranslation (Variables|/Game/CCGToolkit/Blueprints/Widgets/Gameplay/CardWidget.CardWidget_C|GetMoveComponent (Variables|Default|GetCardInHand)) (Math|Vector2D|MakeVector2D (- _x_2 (/ _x 2.0)) (+ (* _y -1.0) _y_2)))
      (Default|OpenGate _cardinhand_2 (Variables|/Game/CCGToolkit/Blueprints/Widgets/Gameplay/CardWidget.CardWidget_C|GetHomeTransform _cardinhand_2) _cardinhand_2 1e+01 "NewEnumerator0")
      (Widget|SetVisibility _cardinhand_2 "Visible"))))