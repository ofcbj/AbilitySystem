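; Ability projectile that delivers a gameplay effect to hostile characters it overlaps.
; On spawn it attaches a particle emitter to its sphere and destroys itself after a short fixed lifetime.
; On overlap it asks the instigator character whether the other character is hostile, then applies the stored effect spec to that target and destroys itself.
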(event EventBeginPlay
  (Effects|SpawnEmitterAttached (Variables|Default|GetParticle) (Variables|Default|GetSphere) "None")
  (Utilities|FlowControl|Delay 3.0)
  (Actor|DestroyActor))

(event Collision|EventActorBeginOverlap
  (params (OtherActor :type Actor%20Object%20Reference))
  (bind _asbp_character_base (Utilities|Casting|CastToBP_CharacterBase OtherActor))
  (bind _asbp_character_base_2 (Utilities|Casting|CastToBP_CharacterBase (Game|GetInstigator)))
  (if (Class|CharacterBase|IsOtherHostile _asbp_character_base_2 _asbp_character_base)
    (Class|CharacterBase|ApplyGESpecHandletoTargetDataSpecHandle _asbp_character_base (Variables|Default|GetEffectSpecHandleFromAbility) (Ability|TargetData|AbilityTargetDatafromActor _asbp_character_base))
    (Actor|DestroyActor)))

(event EventTick
  (params (DeltaSeconds :type Float%20%28single-precision%29)))

(fn ConstructionScript)