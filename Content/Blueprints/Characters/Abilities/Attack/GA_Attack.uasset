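; GA_Attack is a gameplay ability that plays the owning character's attack montage and delivers both melee and ranged attacks.
; While it plays, gameplay events raise a combo counter, apply the character's AttackEffect to melee targets, or spawn a projectile carrying that effect.
; The combo count is passed as the effect level, and the ability ends when the montage completes, blends out or is interrupted.
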(event Ability|EventActivateAbility
  (bind _returnvalue (Ability|GetActorInfo))
  (Ability|CommitAbility)
  (Variables|Default|SetCombo 0)
  (bind _asbp_character_base (Utilities|Casting|CastToBP_CharacterBase (.owneractor _returnvalue)))
  (Animation|Montage|PlayMontage (.skeletalmeshcomponent _returnvalue) (Variables|/Game/Blueprints/Characters/BP_CharacterBase.BP_CharacterBase_C|GetAttackMontage _asbp_character_base)
    (:then
      (Ability|Tasks|WaitGameplayEvent "(TagName=\"skill.combo.increaseCombo\")" 0
        (:then
          (bind _payload (Ability|Tasks|WaitGameplayEvent "(TagName=\"skill.melee.dealDamage\")" 0)
            (:then
              (Ability|Tasks|WaitGameplayEvent "(TagName=\"skill.range.fire\")" 0
                (:EventReceived
                  (bind (_tm _particle) (Default|GetProjectileInfo _asbp_character_base))
                  (Game|SpawnActorfromClass "/Game/Blueprints/Characters/Abilities/Attack/BP_Projectile.BP_Projectile_C" _tm "Undefined" 0 (Ability|MakeOutgoingGameplayEffectSpec (Variables|/Game/Blueprints/Characters/BP_CharacterBase.BP_CharacterBase_C|GetAttackEffect _asbp_character_base) (Math|Conversions|ToFloat(Integer) (Variables|Default|GetCombo))) _particle _asbp_character_base))))
            (:EventReceived
              (GameplayEffects|ApplyGameplayEffectToTarget (Ability|TargetData|AbilityTargetDatafromActor (.Target (Utilities|Struct|BreakGameplayEventData _payload))) (Variables|/Game/Blueprints/Characters/BP_CharacterBase.BP_CharacterBase_C|GetAttackEffect _asbp_character_base) (Variables|Default|GetCombo) 1))))
        (:EventReceived
          (Utilities|IncreaseCombo))))
    (:OnCompleted
      (Ability|EndAbility :!label _label))
    (:OnBlendOut
      (goto _label))
    (:OnInterrupted
      (goto _label))))

(event Ability|EventOnEndAbility
  (params (bWasCancelled :type Boolean)))