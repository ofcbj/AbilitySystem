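; GA_GroundBlast is a Gameplay Ability for a ground-targeted blast that damages or affects, then knocks back, characters in the selected area.
; Activation sets the controller's targeting flag and waits for user confirmation through BP_TargetActorGroundSelect.
; Valid data spawns the blast particle, clears the flag and applies GE_GroundBlast to each targeted actor.
; Characters are pushed away from the player's looking point and briefly stunned.
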(event Ability|EventActivateAbility
  (|CallParentFunction)
  (bind _playercontrollerbase (CallFunction|GetPlayerActorandController))
  (Variables|/Game/Blueprints/Characters/BP_PlayerController.BP_PlayerController_C|SetTargeting _playercontrollerbase true)
  (bind _data (|WaitTargetData :ConfirmationType "UserConfirmed" :Class "/Game/Blueprints/Characters/Abilities/GroundBlast/BP_TargetActorGroundSelect.BP_TargetActorGroundSelect_C" :ReticleClass 0)
    (:ValidData
      (Effects|SpawnEmitteratLocation "/Game/Blueprints/Characters/Abilities/GroundBlast/P_GroundBlast.P_GroundBlast" (Class|AbilitySystemBlueprintLibrary|GetTargetDataEndPoint _data (- (Ability|TargetData|GetDataCountfromTargetData _data) 1)))
      (bind (_characterbase _playercontrollerbase_2) (CallFunction|GetPlayerActorandController))
      (Variables|/Game/Blueprints/Characters/BP_PlayerController.BP_PlayerController_C|SetTargeting _playercontrollerbase_2 false)
      (bind _returnvalue (Class|CharacterBase|GetLookingPoint _characterbase))
      (Variables|Default|SetCenter _returnvalue)
      (for _array_element (Ability|TargetData|GetActorsfromTargetData _data)
        (GameplayEffects|ApplyGameplayEffectToTarget (Ability|TargetData|AbilityTargetDatafromActor _array_element) "/Game/Blueprints/Characters/Abilities/GroundBlast/GE_GroundBlast.GE_GroundBlast_C" 1 1)
        (bind _asbp_character_base (Utilities|Casting|CastToBP_CharacterBase _array_element))
        (Default|PushCharacter _asbp_character_base (Math|Vector|Normalize (- (Transformation|GetActorLocation _asbp_character_base) (Variables|Default|GetCenter))) 5e+02 1.0)))))

(event Ability|EventOnEndAbility
  (params (bWasCancelled :type Boolean))
  (|CallParentFunction bWasCancelled) ; 지금 이 노드는 비활성 상태입니다. \n핀을 끌어서 다른 노드를 연결하면 활성화됩니다.
)