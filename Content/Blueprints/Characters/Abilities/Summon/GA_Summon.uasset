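; GA_Summon is a Gameplay Ability that summons an AI actor from the player's current card at a ground location the player picks.
; Activation flags the controller as targeting and waits for user-confirmed data from BP_TargetActorGroundSelect.
; On valid data it clears the flag, looks up the card's Summon class in BasicSet_DataTable and spawns it facing the character's direction.
; The spawned actor gets SetAI, then the ability ends; cancelled targeting is not handled.
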(event Ability|EventActivateAbility
  (bind (_characterbase _playercontrollerbase) (CallFunction|GetPlayerActorandController))
  (Variables|/Game/Blueprints/Characters/BP_PlayerController.BP_PlayerController_C|SetTargeting _playercontrollerbase true)
  (|WaitTargetData :ConfirmationType "UserConfirmed" :Class "/Game/Blueprints/Characters/Abilities/Common/BP_TargetActorGroundSelect.BP_TargetActorGroundSelect_C" :ReticleClass 0
    (:ValidData
      (bind _playercontrollerbase_2 (CallFunction|GetPlayerActorandController))
      (Variables|/Game/Blueprints/Characters/BP_PlayerController.BP_PlayerController_C|SetTargeting _playercontrollerbase_2 false)
      (bind _returnvalue (Utilities|GetDataTableRow "/Game/CCGToolkit/CardGame/CardSets/Basic_Set/BasicSet_DataTable.BasicSet_DataTable" (Variables|/Game/Blueprints/Characters/BP_PlayerControllerCard.BP_PlayerControllerCard_C|GetCurPlayCard _playercontrollerbase))
        (:then
          (bind _returnvalue_2 (Game|SpawnActorfromClass (.Summon (Utilities|Struct|BreakCard_Struct _returnvalue)) (Math|Transform|MakeTransform (CallFunction|GetPickingLocation) (Transformation|GetActorRotation _characterbase)) "AlwaysSpawn" 0 0))
          (Default|SetAI _returnvalue_2)
          (Ability|EndAbility))))))