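; Gameplay ability for Shinbi's lazer attack, which commits, shows a UI cooldown and plays the start montage section.
; It spawns BP_Lazer on the mesh's Lazer socket and enables camera-controlled rotation.
; Damage events carrying target data apply the damage effect and push hit characters along the caster's forward vector with a brief stun.
; Ending the ability removes mana-drain effects, destroys the lazer and restores rotation control.
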(event Ability|EventActivateAbility
  (|CallParentFunction)
  (Ability|CommitAbility)
  (CallFunction|DoUICooldown)
  (|PlayMontageandWaitProxy "None" "/Game/Blueprints/Characters/Animation/AM_Shinbi_Lazer.AM_Shinbi_Lazer" 1.0 "Start" true 1.0 0.0
    (:then
      (bind _characterbase (CallFunction|GetPlayerActorandController))
      (bind _spawnedactor (|SpawnActor :Class "/Game/Blueprints/Characters/Abilities/Lazer/BP_Lazer.BP_Lazer_C" :Instigator _characterbase)
        (:Success
          (bind _output_get (Variables|Default|SetLazerActor _spawnedactor))
          (Transformation|AttachComponentToComponent _output_get (Variables|/Script/Engine.Character|GetMesh _characterbase) "Lazer" "KeepWorld" "SnapToTarget" "KeepRelative" true)
          (Default|MakeCameraControlRotaation _characterbase true)
          (bind _payload (Ability|Tasks|WaitGameplayEvent "(TagName=\"skill.lazer.dealDamage\")" 0)
            (:EventReceived
              (GameplayEffects|ApplyGameplayEffectToTarget (.TargetData (Utilities|Struct|BreakGameplayEventData _payload)) "/Game/Blueprints/Characters/Abilities/Lazer/GE_Lazer_Damage.GE_Lazer_Damage_C" 1 1)
              (for _array_element (Ability|TargetData|GetActorsfromTargetData (.TargetData (Utilities|Struct|BreakGameplayEventData _payload)))
                (bind _asbp_character_base (Utilities|Casting|CastToBP_CharacterBase _array_element))
                (bind _characterbase_2 (CallFunction|GetPlayerActorandController))
                (Default|PushCharacter _asbp_character_base (Transformation|GetActorForwardVector _characterbase_2) 5e+02 0.2)))))))))

(event Ability|EventOnEndAbility
  (params (bWasCancelled :type Boolean))
  (|CallParentFunction bWasCancelled)
  (Ability|RemoveGameplayEffectFromOwnerWithAssetTags "(GameplayTags=((TagName=\"skill.lazer.drainMana\")))")
  (Actor|DestroyActor (Variables|Default|GetLazerActor))
  (bind _characterbase (CallFunction|GetPlayerActorandController))
  (Default|MakeCameraControlRotaation _characterbase false))