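; BP_Enemy is an enemy character that arms itself with a spiked club on BeginPlay and reports its death to the game mode.
; EquipWeapon destroys any current weapon, resolves a skeletal mesh from a path string through the Asset Registry, and attaches it as a spawned SkeletalMeshActor to the right-hand weapon socket.
; OnDie calls IncreaseNPCKillCount on BP_Gamemode.
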(event EventBeginPlay
  (|CallParentFunction)
  (CallFunction|EquipWeapon "/Game/Weapons/Blunt_SpikedClub/SK_Blunt_SpikedClub.SK_Blunt_SpikedClub"))

(fn ConstructionScript)

(fn EquipWeapon
  (params (AssetPath :type String))
  (Utilities|IsValid (Variables|Default|GetWeaponActor)
    (:Is%20Valid
      (Actor|DestroyActor (Variables|Default|GetWeaponActor)))
    (:Is%20Not%20Valid
      _))
  (bind _returnvalue (Class|AssetRegistry|GetAssetbyObjectPath (Class|AssetRegistryHelpers|GetAssetRegistry) (Utilities|String|StringToName AssetPath) false))
  (bind _asskeletal_mesh (Utilities|Casting|CastToSkeletalMesh (Class|AssetRegistryHelpers|GetAsset _returnvalue)))
  (if (Utilities|IsValid _asskeletal_mesh)
    (bind _returnvalue_2 (Class|MovieSceneTransformOrigin|GetTransformOrigin(Message) (Variables|Character|GetCharacterMovement)))
    (bind _returnvalue_3 (Game|SpawnActorfromClass "/Script/Engine.SkeletalMeshActor" _returnvalue_2 "Undefined" 0 0))
    (Variables|Default|SetWeaponActor _returnvalue_3)
    (Class|SkinnedMeshComponent|SetSkeletalMesh (Variables|/Script/Engine.SkeletalMeshActor|GetSkeletalMeshComponent _returnvalue_3) _asskeletal_mesh true)
    (Transformation|AttachComponentToComponent _returnvalue_3 (Variables|Character|GetMesh) "b_MF_Weapon_R" "SnapToTarget" "SnapToTarget" "KeepWorld" true)))

(fn OnDie
  (bind _asbp_gamemode (Utilities|Casting|CastToBP_Gamemode (Game|GetGameMode)))
  (Default|IncreaseNPCKillCount _asbp_gamemode 0.0))