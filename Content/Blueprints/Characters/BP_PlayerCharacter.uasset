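; BP_PlayerCharacter is the player's character, built on gameplay abilities, which it acquires on BeginPlay while hiding its own health bar.
; Health and mana changes update the orb percentages in BP_PlayerController's primary UI.
; Capsule overlaps with hostile characters send a dash-damage gameplay event to itself once per target, tracked in an exclusion list.
; On death it plays a montage, waits its duration, then destroys itself.
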(event OnComponentBeginOverlap(CapsuleComponent)
  (params (OverlappedComponent :type Primitive%20Component%20Object%20Reference) (OtherActor :type Actor%20Object%20Reference) (OtherComp :type Primitive%20Component%20Object%20Reference) (OtherBodyIndex :type Integer) (bFromSweep :type Boolean) (SweepResult :type Hit%20Result%20Structure%20%28by%20ref%29))
  (bind _self self)
  (bind _overlapexclude (Variables|Default|GetOverlapExclude))
  (bind _ascharacter_base (Utilities|Casting|CastToCharacterBase OtherActor))
  (Class|CharacterBase|IsOtherHostile _ascharacter_base)
  (if true
    (if (not (Utilities|Array|ContainsItem _overlapexclude OtherActor))
      (Utilities|Array|AddUnique _overlapexclude OtherActor)
      (Ability|SendGameplayEventtoActor _self "(TagName=\"skill.dash.dealDamage\")" (Utilities|Struct|MakeGameplayEventData "(TagName=\"skill.dash.dealDamage\")" _self OtherActor)))))

(event EventOnManaChanged
  (params (Mana :type Float%20%28single-precision%29) (MaxMana :type Float%20%28single-precision%29))
  (bind _asbp_player_controller (Utilities|Casting|CastToBP_PlayerController (Game|GetPlayerController 0)))
  (Default|SetPercentage (Variables|/Game/UI/WBP_PrimaryUI.WBP_PrimaryUI_C|GetManaBall (Variables|/Game/Blueprints/Characters/BP_PlayerController.BP_PlayerController_C|GetPrimaryUI _asbp_player_controller)) (/ Mana MaxMana)))

(event Collision|EventActorBeginOverlap
  (params (OtherActor :type Actor%20Object%20Reference))
  (|CallParentFunction OtherActor) ; 지금 이 노드는 비활성 상태입니다. \n핀을 끌어서 다른 노드를 연결하면 활성화됩니다.
)

(event EventTick
  (params (DeltaSeconds :type Float%20%28single-precision%29))
  (|CallParentFunction DeltaSeconds) ; 지금 이 노드는 비활성 상태입니다. \n핀을 끌어서 다른 노드를 연결하면 활성화됩니다.
)

(event EventOnHealthChanged
  (params (Health :type Float%20%28single-precision%29) (MaxHealth :type Float%20%28single-precision%29))
  (bind _asbp_player_controller (Utilities|Casting|CastToBP_PlayerController (Game|GetPlayerController 0)))
  (Default|SetPercentage (Variables|/Game/UI/WBP_PrimaryUI.WBP_PrimaryUI_C|GetHealthBall (Variables|/Game/Blueprints/Characters/BP_PlayerController.BP_PlayerController_C|GetPrimaryUI _asbp_player_controller)) (/ Health MaxHealth)))

(event EventDie
  (bind _returnvalue (Animation|PlayAnimMontage "/Game/Blueprints/Characters/Animation/AM_Shinbi_Die.AM_Shinbi_Die" 1.0 "None"))
  (Utilities|FlowControl|Delay _returnvalue)
  (Actor|DestroyActor))

(event EventBeginPlay
  (|CallParentFunction)
  (Rendering|SetVisibility (Variables|Default|GetHealthBar) false false)
  (Class|CharacterBase|AcquireAbilities (Variables|Default|GetInitialAbilities)))

(fn ConstructionScript
  (|CallParentFunction))