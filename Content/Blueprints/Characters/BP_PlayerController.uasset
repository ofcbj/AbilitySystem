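; Player controller that creates the primary UI and handles camera-relative movement, jump, look, and a primary action that either confirms ability targeting or attacks.
; SwitchCharacter cycles possession through the GameMode's player character list, handing the old pawn to AI and stopping the next one's AI logic.
; A test input spawns an AI BP_Boris at the picking point.
; Ability-slot activation calls are unwired, and the action gate always returns true.
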(event EventBeginPlay
  (bind _returnvalue (UserInterface|CreateWidget "/Game/UI/WBP_PrimaryUI.WBP_PrimaryUI_C"))
  (bind _output_get (Variables|Default|SetPrimaryUI _returnvalue))
  (UserInterface|Viewport|AddtoViewport _output_get 0))

(event EventTick
  (params (DeltaSeconds :type Float%20%28single-precision%29)))

(event EventAddAbilitytoUI
  (params (AbilityInfo :type Gameplay%20Ability%20Info%20Structure)))

(event Input|ActionEvents|InputActionJump
  (params (Key :type Key%20Structure :default "None"))
  ;[1 1 1] Base Controll
  (:Pressed
    (if (CallFunction|IsEnableAction)
      (bind _ascharacter (Utilities|Casting|CastToCharacter (Pawn|GetControlledPawn)))
      (Character|Jump _ascharacter))))

(event Input|ActionEvents|InputActionSlot4
  (params (Key :type Key%20Structure :default "None")))

(event Input|ActionEvents|InputActionChangeCharacter
  (params (Key :type Key%20Structure :default "None"))
  (:Pressed
    (CallFunction|SwitchCharacter)))

(event Input|ActionEvents|InputActionPrimaryAction
  (params (Key :type Key%20Structure :default "None"))
  (:Pressed
    (bind _asbp_character_base (Utilities|Casting|CastToBP_CharacterBase (Pawn|GetControlledPawn)))
    (if (Variables|Default|GetTargeting)
      (Class|AbilitySystemComponent|TargetConfirm (Variables|/Script/AbilitySystem.CharacterBase|GetAbilitySystemComp _asbp_character_base))
      (elif (CallFunction|IsEnableAction)
        (Default|Attack _asbp_character_base)))))

(event Input|ActionEvents|InputActionSlot5
  (params (Key :type Key%20Structure :default "None")))

(event Input|ActionEvents|InputActionSlot1
  (params (Key :type Key%20Structure :default "None")))

(event Input|ActionEvents|InputActionSlot2
  (params (Key :type Key%20Structure :default "None")))

(event Input|ActionEvents|InputActionSlot3
  (params (Key :type Key%20Structure :default "None")))

(event Input|ActionEvents|InputActionTest
  (params (Key :type Key%20Structure :default "None"))
  (:Pressed
    (bind _returnvalue (Game|SpawnActorfromClass "/Game/Blueprints/Characters/BP_Boris.BP_Boris_C" (Math|Conversions|ToTransform(Vector) (CallFunction|GetPickingPoint)) "Undefined" 0 0))
    (Default|SetAI _returnvalue)))

(event Input|AxisEvents|InputAxisMoveForward
  (params (AxisValue :type Float%20%28single-precision%29))
  ;[1 1 1] Base Controll
  (if (CallFunction|IsEnableAction)
    (Pawn|Input|AddMovementInput (Pawn|GetControlledPawn) (Math|Vector|GetForwardVector (Camera|GetCameraRotation (Game|GetPlayerCameraManager 0))) AxisValue false)))

(event Input|AxisEvents|InputAxisMoveRight
  (params (AxisValue :type Float%20%28single-precision%29))
  ;[1 1 1] Base Controll
  (if (CallFunction|IsEnableAction)
    (Pawn|Input|AddMovementInput (Pawn|GetControlledPawn) (Math|Vector|GetRightVector (Camera|GetCameraRotation (Game|GetPlayerCameraManager 0))) AxisValue false)))

(event Input|AxisEvents|InputAxisLookUp
  (params (AxisValue :type Float%20%28single-precision%29))
  ;[1 1 1] Base Controll
  (Class|PlayerController|AddPitchInput AxisValue))

(event Input|AxisEvents|InputAxisLookRight
  (params (AxisValue :type Float%20%28single-precision%29))
  ;[1 1 1] Base Controll
  (Class|PlayerController|AddYawInput AxisValue))

(fn ConstructionScript)

(fn TryActivateAbilityUISlot
  (params (SlotNumber :type Integer))
  (bind (_abilityclass _valid) (Default|GetSlotAbilityClass (Variables|Default|GetPrimaryUI) SlotNumber))
  (if _valid
    (bind _asbp_player_character (Utilities|Casting|CastToBP_PlayerCharacter (Pawn|GetControlledPawn)))
    (Abilities|TryActivateAbilitybyClass (Variables|/Script/AbilitySystem.CharacterBase|GetAbilitySystemComp _asbp_player_character) _abilityclass false)))

(fn DrawCard
  (params (CardName :type String))
  (Default|AddCardWidget (Variables|/Game/UI/WBP_PrimaryUI.WBP_PrimaryUI_C|GetCardManager (Variables|Default|GetPrimaryUI)) (Utilities|String|StringToName CardName) "NewEnumerator0"))

(fn IsEnableAction
  (return true))

(fn PlayCard
  (params (CardName :type Name)))

(fn SwitchCharacter
  (bind _gamemode (CallFunction|GetGameModeBP))
  (bind _playercharacterlist (Variables|/Game/Blueprints/BP_GameMode.BP_Gamemode_C|GetPlayerCharacterList _gamemode))
  (for (_array_element _array_index) _playercharacterlist
    (if (== _array_element (Pawn|GetControlledPawn))
      (LocalVariables|SetCurPlayerCharacterIndex _array_index)))
  (if (== (LocalVariables|GetCurPlayerCharacterIndex) (- (Utilities|Array|Length _playercharacterlist) 1))
    (LocalVariables|SetChangePlayerCharacterIndex 0)
    (else
      (LocalVariables|SetChangePlayerCharacterIndex (+ (LocalVariables|GetCurPlayerCharacterIndex) 1))))
  (bind _output_get (LocalVariables|SetPrevControlledPawn (Pawn|GetControlledPawn)))
  (Pawn|UnPossess)
  (bind _asbp_player_character (Utilities|Casting|CastToBP_PlayerCharacter _output_get))
  (Default|SetAI _asbp_player_character)
  (Default|SyncUI _asbp_player_character)
  (AI|Logic|StopLogic (Variables|/Script/AIModule.AIController|GetBrainComponent (Variables|/Game/Blueprints/Characters/BP_PlayerCharacter.BP_PlayerCharacter_C|GetAIController (Utilities|Array|Get(acopy) _playercharacterlist (LocalVariables|GetChangePlayerCharacterIndex)))) "Switch")
  (Pawn|UnPossess (Variables|/Game/Blueprints/Characters/BP_PlayerCharacter.BP_PlayerCharacter_C|GetAIController (Utilities|Array|Get(acopy) _playercharacterlist (LocalVariables|GetChangePlayerCharacterIndex))))
  (Pawn|Possess (Utilities|Array|Get(acopy) _playercharacterlist (LocalVariables|GetChangePlayerCharacterIndex)))
  (Default|SyncUI (Utilities|Array|Get(acopy) _playercharacterlist (LocalVariables|GetChangePlayerCharacterIndex))))