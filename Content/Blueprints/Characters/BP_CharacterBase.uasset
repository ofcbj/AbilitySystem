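; Base character Blueprint built on the Gameplay Ability System, providing melee, dash, health regen, knockback and death.
; It acquires melee on BeginPlay, exposes events that activate abilities by class, and turns sword overlaps into damage gameplay events sent to itself with the target.
; Health changes update a widget health bar, and death plays a montage before destroying the actor.
; Knockback briefly zeroes ground friction around an impulse, with optional hit stun.
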(event OnComponentBeginOverlap(SwordCollider)
  (params (OverlappedComponent :type Primitive%20Component%20Object%20Reference) (OtherActor :type Actor%20Object%20Reference) (OtherComp :type Primitive%20Component%20Object%20Reference) (OtherBodyIndex :type Integer) (bFromSweep :type Boolean) (SweepResult :type Hit%20Result%20Structure%20%28by%20ref%29))
  (if (!= OtherActor self)
    (Ability|SendGameplayEventtoActor self "(TagName=\"skill.melee.dealDamage\")" (Utilities|Struct|MakeGameplayEventData "" 0 OtherActor 0 0 "()" "(GameplayTags=)" "(GameplayTags=)" 0.0 (Ability|TargetData|AbilityTargetDatafromActor OtherActor)))))

(event Custom|PushCharacter
  (params (ImpulseDirection :type Vector) (PushStrength :type Float%20%28single-precision%29) (StunDuration :type Float%20%28single-precision%29))
  (bind _charactermovement (Variables|Character|GetCharacterMovement))
  (Variables|Default|SetDefaultGroundFriction (Variables|/Script/Engine.CharacterMovementComponent|GetGroundFriction _charactermovement))
  (Variables|/Script/Engine.CharacterMovementComponent|SetGroundFriction _charactermovement 0.0)
  (Physics|AddImpulse _charactermovement (* ImpulseDirection PushStrength) true)
  (if (> StunDuration 0.0)
    (Class|CharacterBase|HitStun StunDuration))
  (Utilities|FlowControl|Delay 0.3)
  (Variables|/Script/Engine.CharacterMovementComponent|SetGroundFriction _charactermovement (Variables|Default|GetDefaultGroundFriction)))

(event Custom|TryHealthRegen
  (Abilities|TryActivateAbilitybyClass (Variables|Default|GetAbilitySystemComp) "/Game/Blueprints/Characters/Abilities/HealthRegen/GA_HealthRegen.GA_HealthRegen_C" true))

(event Custom|TryDash
  (Abilities|TryActivateAbilitybyClass (Variables|Default|GetAbilitySystemComp) "/Game/Blueprints/Characters/Abilities/Dash/GA_Dash.GA_Dash_C" true))

(event Custom|MeleeAttack
  (Abilities|TryActivateAbilitybyClass (Variables|Default|GetAbilitySystemComp) "/Game/Blueprints/Characters/Abilities/Melee/GA_Melee.GA_Melee_C" true))

(event EventBeginPlay
  (Class|CharacterBase|AcquireAbility "/Game/Blueprints/Characters/Abilities/Melee/GA_Melee.GA_Melee_C"))

(event Collision|EventActorBeginOverlap
  (params (OtherActor :type Actor%20Object%20Reference)))

(event EventTick
  (params (DeltaSeconds :type Float%20%28single-precision%29)))

(event EventOnHealthChanged
  (params (Health :type Float%20%28single-precision%29) (MaxHealth :type Float%20%28single-precision%29))
  (bind _ashealth_bar (Utilities|Casting|CastToHealthBar (UserInterface|GetUserWidgetObject (Variables|Default|GetHealthBar))))
  (Default|SetPercentage _ashealth_bar (/ Health MaxHealth)))

(event EventDie
  (bind _returnvalue (Animation|PlayAnimMontage "/Game/Blueprints/Characters/Animation/AM_Shinbi_Die.AM_Shinbi_Die" 1.0 "None"))
  (Utilities|FlowControl|Delay _returnvalue)
  (Actor|DestroyActor))

(fn ConstructionScript)

(fn SetCollisiontoPawn
  (params (NewResponse :type ECollisionResponse%20Enum :default "ECR_Ignore"))
  (Collision|SetCollisionResponsetoChannel (Variables|Default|GetCapsuleComponent) "ECC_Pawn" NewResponse))