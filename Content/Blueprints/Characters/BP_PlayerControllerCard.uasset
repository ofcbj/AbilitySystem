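; Player controller for a wave-based card game that fills the hand and plays cards as character abilities.
; FillHand picks up to ten BasicSet data table rows (the first five plus a six-row slice for the current wave), deals them with staggered delays, then enables the card phase UI.
; PlayCard activates GA_Summon for hero cards and a name-matched ability for spells.
; IsEnableAction returns true only outside the card phase.
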(event Custom|FillHand
  (bind _gamemode (CallFunction|GetGameModeBP))
  (bind _primaryui (Variables|Default|GetPrimaryUI))
  (bind _cardlist (Variables|Default|GetCardList))
  (bind _cardmanager (Variables|/Game/UI/WBP_PrimaryUI.WBP_PrimaryUI_C|GetCardManager _primaryui))
  (bind _currentwave (Variables|/Game/Blueprints/BP_GameMode.BP_GameMode_C|GetCurrentWave _gamemode))
  (bind _returnvalue (- _currentwave 1))
  (bind _returnvalue_2 (* _returnvalue 6))
  (Default|RemoveCardWidgetfromHand _cardmanager 0 0 true)
  (Widget|SetVisibility _cardmanager "Visible")
  (Utilities|Array|Clear (Variables|Default|GetCardList))
  (bind _outrownames (DataTable|GetDataTableRowNames "/Game/CCGToolkit/CardGame/CardSets/Basic_Set/BasicSet_DataTable.BasicSet_DataTable"))
  (bind (_array_element _array_index) (Utilities|Array|ForEachLoopwithBreak _outrownames :!label _label)
    (:LoopBody
      (if (>= (Utilities|Array|Length (Variables|Default|GetCardList)) 10)
        (goto _label Break)
        (elif (or (and (>= _array_index 0) (< _array_index 5)) (and (>= _array_index (+ _returnvalue_2 5)) (< _array_index (+ (+ _returnvalue_2 6) 5))))
          (Utilities|Array|Add _cardlist _array_element))))
    (:Completed
      (bind _arrayelement (Utilities|ForEachLoopDelayed _cardlist 1 0.2)
        (:LoopBody
          (CallFunction|DrawCard _arrayelement))
        (:Completed
          (Variables|/Game/Blueprints/BP_GameMode.BP_GameMode_C|SetIsCardPlay (CallFunction|GetGameModeBP) true)
          (Variables|Default|SetbShowMouseCursor true)
          (Widget|SetVisibility (Variables|/Game/UI/WBP_PrimaryUI.WBP_PrimaryUI_C|GetStartButton (Variables|Default|GetPrimaryUI)) "Visible"))))))

(event EventBeginPlay
  (|CallParentFunction))

(event EventTick
  (params (DeltaSeconds :type Float%20%28single-precision%29))
  (|CallParentFunction DeltaSeconds) ; 지금 이 노드는 비활성 상태입니다. \n핀을 끌어서 다른 노드를 연결하면 활성화됩니다.
)

(fn ConstructionScript
  (|CallParentFunction))

(fn IsEnableAction
  (return (not (Variables|/Game/Blueprints/BP_GameMode.BP_GameMode_C|GetIsCardPlay (CallFunction|GetGameModeBP)))))

(fn PlayCard
  (params (CardName :type Name :default "None"))
  (bind _playercharacter (CallFunction|GetPlayerCharacterBP))
  (bind _output_get (Variables|Default|SetCurPlayCard CardName))
  (bind _returnvalue (Utilities|GetDataTableRow "/Game/CCGToolkit/CardGame/CardSets/Basic_Set/BasicSet_DataTable.BasicSet_DataTable" _output_get)
    (:then
      (switch Utilities|FlowControl|Switch|SwitchonCardType_Enum (.Type (Utilities|Struct|BreakCard_Struct _returnvalue))
        (:NewEnumerator6
          (Abilities|TryActivateAbilitybyClass (Variables|/Script/AbilitySystem.CharacterBase|GetAbilitySystemComp _playercharacter) "/Game/Blueprints/Characters/Abilities/Summon/GA_Summon.GA_Summon_C" false))
        (:NewEnumerator1
          (Default|UseAbility _playercharacter (Utilities|String|ToString(Name) CardName)))))))

(fn DrawCard
  (params (CardName :type Name))
  (Default|AddCardWidget (Variables|/Game/UI/WBP_PrimaryUI.WBP_PrimaryUI_C|GetCardManager (Variables|Default|GetPrimaryUI)) CardName "NewEnumerator0"))